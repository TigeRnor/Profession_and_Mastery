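; Consumable warpaint game item that applies the paint set by its WarpaintID to the character using it, with ID 0 noted as washing it off.
; On use it writes that index into the face, body and hands texture slots and the warpaint tint of the character layout.
; It then records a server-only Warpaint journey event, adding BuffWarpaint for a middle range of IDs, before running the parent use logic.
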(event EventOnUseItem
  (params (invokingCharacter :type Conan%20Character%20Object%20Reference))
  (CallFunction|UpdateCharacterLayout invokingCharacter (Variables|Default|GetWarpaintID))
  (CallFunction|UpdateJourneyEvent invokingCharacter)
  (|CallParentFunction invokingCharacter))

(fn UpdateJourneyEvent
  (params (InvokingCharacter :type Character%20Object%20Reference))
  (if (Networking|IsServer)
    (bind _asbase_player_char_interface (Utilities|Casting|CastToBasePlayerCharInterface InvokingCharacter))
    (LocalVariables|SetBasePlayerCharInterface _asbase_player_char_interface)
    (switch int (Variables|Default|GetWarpaintID) ; 0 = wash it off.
      (:Default
        (Default|AddJourneyEventInterfaceCall (LocalVariables|GetBasePlayerCharInterface) "Warpaint" :!label _label))
      (:1
        (goto _label))
      (:2
        (goto _label))
      (:3
        (goto _label))
      (:4
        (goto _label))
      (:5
        (goto _label))
      (:6
        (goto _label))
      (:7
        (goto _label))
      (:8
        (Default|AddJourneyEventInterfaceCall (LocalVariables|GetBasePlayerCharInterface) "Warpaint" :!label _label_2)
        (Default|AddJourneyEventInterfaceCall (LocalVariables|GetBasePlayerCharInterface) "BuffWarpaint"))
      (:9
        (goto _label_2))
      (:10
        (goto _label_2))
      (:11
        (goto _label_2))
      (:12
        (goto _label_2))
      (:13
        (goto _label_2))
      (:14
        (goto _label_2))
      (:15
        (goto _label))
      (:16
        (goto _label)))))

(fn UpdateCharacterLayout
  (params (InvokingCharacter :type Object%20Object%20Reference) (WarpaintIndex :type Integer))
  (bind _character_layout (Class|IHasCharacterLayoutInterface|GetCharacterLayout(Message) InvokingCharacter))
  (bind _output_get (Variables|Default|SetLayout _character_layout))
  (Class|CharacterFunctionLibrary|SetCharacterTextureSlot (.texturelayout _output_get) "WarpaintFace" WarpaintIndex)
  (Class|CharacterFunctionLibrary|SetCharacterTextureSlot (.texturelayout _output_get) "WarpaintBody" WarpaintIndex)
  (Class|CharacterFunctionLibrary|SetCharacterTextureSlot (.texturelayout _output_get) "WarpaintHands" WarpaintIndex)
  (Class|CharacterFunctionLibrary|SetCharacterTintSlot (.tintlayout _output_get) "Warpaint" WarpaintIndex)
  (Class|IHasCharacterLayoutInterface|SetCharacterLayout(Message) InvokingCharacter (Variables|Default|GetLayout)))