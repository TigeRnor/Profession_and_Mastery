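; Buff Blueprint for the Duelist's Berserk warcry, which modifies the owning character's Might attribute.
; On start it calls the parent effect, then makes two identical additive Might modifier calls of twice BuffPotency, using Merge mode on the default modifier ID.
; On clear it repeats both calls with the value multiplied to zero rather than removing the modifier.
; StartBuff only forwards to the parent.
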(event EventBeginPlay)

(event EventTick
  (params (DeltaSeconds :type Float%20%28single-precision%29)))

(event EventGameplayEffecttoApplyonBuffStart
  (bind _owningcharacter (Variables|Default|GetOwningCharacter))
  (|CallParentFunction)
  (Class|ConanCharacter|AddIntStatModifier _owningcharacter "AttributeMight" "Default" "Add" (* (Variables|Default|GetBuffPotency) 2) "Merge")
  (Class|ConanCharacter|AddIntStatModifier _owningcharacter "AttributeMight" "Default" "Add" (* (Variables|Default|GetBuffPotency) 2) "Merge"))

(event EventGameplayEffecttoApplyonBuffCleared
  (bind _owningcharacter (Variables|Default|GetOwningCharacter))
  (|CallParentFunction)
  (Class|ConanCharacter|AddIntStatModifier _owningcharacter "AttributeMight" "Default" "Add" (* (* (Variables|Default|GetBuffPotency) 2) 0) "Merge")
  (Class|ConanCharacter|AddIntStatModifier _owningcharacter "AttributeMight" "Default" "Add" (* (* (Variables|Default|GetBuffPotency) 2) 0) "Merge"))

(event EventStartBuff
  (params (BuffPotency :type Integer) (DamageCauser :type Actor%20Object%20Reference) (OwningCharacter :type Conan%20Character%20Object%20Reference) (Instigator :type Controller%20Object%20Reference))
  (|CallParentFunction BuffPotency DamageCauser OwningCharacter Instigator))