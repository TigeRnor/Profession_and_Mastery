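; Outlaw Gambit buff, a warcry-type effect described as raising accuracy by 3.
; On start it forces an attack vocal, drains the player's current stamina to zero and ends every buff in WarcryList through the buff system.
; It conditionally swaps the character's voice audio to a warcry sound, then hands off to the parent StartBuff.
; The accuracy bonus appears here only as description text.
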(event EventStartBuff
  (params (BuffPotency :type Integer) (DamageCauser :type Actor%20Object%20Reference) (OwningCharacter :type Conan%20Character%20Object%20Reference) (Instigator :type Controller%20Object%20Reference))
  (bind _asbase_player_char (Utilities|Casting|CastToBasePlayerChar OwningCharacter))
  (CallFunction|VocalsPlayfromSoundName "voc_attack" 0 true (Variables|/Game/Characters/BP_AC_AudioController.BP_AC_AudioController_C|GetVoiceSetType (Actor|GetComponentbyClass _asbase_player_char "/Game/Characters/BP_AC_AudioController.BP_AC_AudioController_C")) "NewEnumerator4")
  (Default|AdjustStaminaCurrent _asbase_player_char (* -1 (Class|ConanCharacter|GetStaminaCurrent _asbase_player_char)))
  (CallFunction|RemoveWarcry OwningCharacter)
  (CallFunction|WarcryVocalize _asbase_player_char)
  (|CallParentFunction BuffPotency DamageCauser OwningCharacter Instigator))

(fn GetEffectDescription
  (return (Utilities|Text|FormatText "Accuracy increased by 3")))

(fn RemoveWarcry
  (params (NewParam :type Object%20Object%20Reference))
  (bind _asbase_player_char (Utilities|Casting|CastToBasePlayerChar NewParam)
    (:then
      (for _array_element (Variables|Default|GetWarcryList)
        (Default|EndBuff (Variables|/Game/Characters/BaseBPCombat.BaseBPCombat_C|Get00_BP_AC_BuffSystem _asbase_player_char) _array_element))
      (return))
    (:CastFailed
      (return))))

(fn WarcryVocalize
  (params (Object :type Object%20Object%20Reference))
  (bind _asbase_bpchar (Utilities|Casting|CastToBaseBPChar Object)
    (:then
      (Utilities|IsValid+Branch (Variables|/Game/Characters/BaseBPChar.BaseBPChar_C|GetVoiceAudioComp _asbase_bpchar) (Class|ConanAudioComponent|IsPlaying (Variables|/Game/Characters/BaseBPChar.BaseBPChar_C|GetVoiceAudioComp _asbase_bpchar))
        (:True
          (Variables|/Script/ConanSandbox.ConanAudioComponent|SetAttenuationSettings (Variables|/Game/Characters/BaseBPChar.BaseBPChar_C|GetVoiceAudioComp _asbase_bpchar) "/Game/Sound/Attenuations/Att_client_voc.Att_client_voc")
          (Variables|/Script/ConanSandbox.ConanAudioComponent|SetConcurrencySettings (Variables|/Game/Characters/BaseBPChar.BaseBPChar_C|GetVoiceAudioComp _asbase_bpchar) 0)
          (Variables|/Script/ConanSandbox.ConanAudioComponent|SetSoundAsset (Variables|/Game/Characters/BaseBPChar.BaseBPChar_C|GetVoiceAudioComp _asbase_bpchar) "/Game/Sound/Voiceover/Female_emotes/Female_1/f1_voc_cry_3.f1_voc_cry_3")
          (Class|ConanAudioComponent|LoadandPlay (Variables|/Game/Characters/BaseBPChar.BaseBPChar_C|GetVoiceAudioComp _asbase_bpchar) 0.0))))
    (:CastFailed
      (Development|PrintString "Hello"))))