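; BP_HazardArea_opium is a spherical hazard area that applies a configurable debuff to players inside it.
; Overlaps track affected players and run a looping timer that reapplies stacked buffs through their BuffSystem component while the hazard is active.
; Trigger messages toggle, reset or set the active state.
; Leaving or switching off removes the debuff unless it is set to linger.
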(event OnComponentBeginOverlap(TriggerSphere)
  (params (OverlappedComponent :type Primitive%20Component%20Object%20Reference) (OtherActor :type Actor%20Object%20Reference) (OtherComp :type Primitive%20Component%20Object%20Reference) (OtherBodyIndex :type Integer) (bFromSweep :type Boolean) (SweepResult :type Hit%20Result%20Structure%20%28by%20ref%29))
  (CallFunction|ActorOverlapBegin OtherActor))

(event OnComponentEndOverlap(TriggerSphere)
  (params (OverlappedComponent :type Primitive%20Component%20Object%20Reference) (OtherActor :type Actor%20Object%20Reference) (OtherComp :type Primitive%20Component%20Object%20Reference) (OtherBodyIndex :type Integer))
  (CallFunction|ActorOverlapEnd OtherActor))

(event Custom|ClearAllBuffs
  (if (not (Variables|HazardArea|GetIsLingeringDebuff))
    (for _array_element (Variables|Default|GetAffected%20Chars)
      (CallFunction|RemoveBuff _array_element))))

(event Custom|Player%20Leaves
  (params (Player :type Actor%20Object%20Reference))
  (Utilities|Array|RemoveItem (Variables|Default|GetAffected%20Chars) Player)
  (if (== (Utilities|Array|Length (Variables|Default|GetAffected%20Chars)) 0)
    (Utilities|Time|ClearandInvalidateTimerbyHandle (Variables|Default|GetTickTimer))))

(event Custom|ActorOverlapEnd
  (params (OtherActor :type Actor%20Object%20Reference))
  (if (== (Utilities|GetClass OtherActor) "/Game/Characters/BasePlayerChar.BasePlayerChar_C")
    (CallFunction|PlayerLeaves OtherActor)
    (if (not (Variables|HazardArea|GetIsLingeringDebuff))
      (CallFunction|RemoveBuff OtherActor))))

(event Custom|Hazard%20Tick
  (if (Variables|HazardArea|GetStateCurrent)
    (for _array_element (Variables|Default|GetAffected%20Chars)
      (CallFunction|ApplyBuff _array_element))))

(event Custom|ActorOverlapBegin
  (params (OtherActor :type Actor%20Object%20Reference))
  (if (== (Utilities|GetClass OtherActor) "/Game/Characters/BasePlayerChar.BasePlayerChar_C")
    (CallFunction|PlayerEnters OtherActor)
    (if (Variables|HazardArea|GetStateCurrent)
      (CallFunction|ApplyBuff OtherActor))))

(event Custom|SetState
  (params (Value :type Boolean))
  (bind _output_get (Variables|HazardArea|SetStateCurrent Value))
  (if (not _output_get)
    (CallFunction|ClearAllBuffs)))

(event Custom|Player%20Enters
  (params (Player :type Actor%20Object%20Reference))
  (Utilities|Array|AddUnique (Variables|Default|GetAffected%20Chars) Player)
  (if (not (Class|KismetSystemLibrary|TimerExistsHandle (Variables|Default|GetTickTimer)))
    (bind _returnvalue (Utilities|Time|SetTimerbyEvent (delegate Custom|Hazard%20Tick) (Variables|HazardArea|GetTick%20Time) true))
    (Variables|Default|SetTickTimer _returnvalue)))

(event EventTrigger
  (params (Data :type STR%20Trigger%20Message%20Structure))
  (switch Utilities|FlowControl|Switch|SwitchonE_TriggerMessage (.message Data)
    (:NewEnumerator0
      (CallFunction|SetState (not (Variables|HazardArea|GetStateCurrent))))
    (:NewEnumerator1
      (CallFunction|SetState (Variables|HazardArea|GetStateDefault)))
    (:NewEnumerator2
      (CallFunction|SetState true))
    (:NewEnumerator3
      (CallFunction|SetState false))))

(fn ConstructionScript
  (bind _trigger_radius (Variables|HazardArea|GetTrigger%20Radius))
  (bind _trigger_sphere (Variables|Components|GetTrigger%20Sphere))
  (Utilities|FlowControl|Sequence
    (:then_0
      (if (!= (Variables|/Script/Engine.SphereComponent|GetSphereRadius _trigger_sphere) _trigger_radius)
        (Components|Sphere|SetSphereRadius _trigger_sphere _trigger_radius true)))
    (:then_1
      (Variables|HazardArea|SetStateCurrent (Variables|HazardArea|GetStateDefault)))))

(fn ApplyBuff
  (params (Player :type Actor%20Object%20Reference))
  (bind _returnvalue (Actor|GetComponentsByClass Player "/Game/Systems/Buffs/00_BP_AC_BuffSystem.00_BP_AC_BuffSystem_C"))
  (if (>= (Utilities|Array|Length _returnvalue) 0)
    (for _index (range 1 (Variables|HazardArea|GetStacks))
      (Default|AddBuff (Utilities|Array|Get(acopy) _returnvalue) (Variables|HazardArea|GetHazard%20Debuff) self (Variables|HazardArea|GetPotency)))))

(fn RemoveBuff
  (params (Player :type Actor%20Object%20Reference))
  (bind _returnvalue (Actor|GetComponentsByClass Player "/Game/Systems/Buffs/00_BP_AC_BuffSystem.00_BP_AC_BuffSystem_C"))
  (if (> (Utilities|Array|Length _returnvalue) 0)
    (Default|RemoveBuff (Utilities|Array|Get(acopy) _returnvalue) (Variables|HazardArea|GetHazard%20Debuff))))