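; AC_OnlineList is a component, going by its name, that keeps a list of online players on the server.
; Every Tick, on a server or dedicated server, it clears the list and rebuilds it from all FunCombat_PlayerController actors.
; Each controller's character name is added uniquely, and guild names from controlled BasePlayerChar pawns go into the same list.
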(event EventBeginPlay)

(event EventTick
  (params (DeltaSeconds :type Float%20%28single-precision%29))
  (if (Networking|IsServer)
    (Utilities|Array|Clear (Variables|Default|GetListOfOnlinePLayers) :!label _label)
    (bind _outactors (Actor|GetAllActorsOfClass "/Game/Systems/FunCombat_PlayerController.FunCombat_PlayerController_C"))
    (for _array_element _outactors
      (Utilities|Array|AddUnique (Variables|Default|GetListOfOnlinePLayers) (Class|ConanPlayerController|GetCharacterName _array_element))
      (bind _asbase_player_char (Utilities|Casting|CastToBasePlayerChar (Pawn|GetControlledPawn _array_element)))
      (Utilities|Array|AddUnique (Variables|Default|GetListOfOnlinePLayers) (Class|Guild|GetGuildName (Class|ConanCharacter|GetGuild _asbase_player_char))))
    (elif (Networking|IsDedicatedServer)
      (goto _label))))