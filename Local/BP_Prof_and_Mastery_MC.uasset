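; Mod controller for a Conan Exiles professions and class mastery mod, injecting its content into the base game's data tables.
; ModDataTableOperations is one flat sequence of MergeDataTables calls covering feats, items, recipes, stat overrides, equipment variations, loot, spawns, thralls, warpaints and journey steps.
; Some merges repeat, and the bare RecipesTable and FeatTable merges have no source table set.
; The construction script and widget function are empty.
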(fn ConstructionScript)

(fn ModDataTableOperations
  (Class|ModController|MergeDataTables "/Game/Items/Feats/FeatTable.FeatTable" "/Game/Mods/Profession_and_Mastery/DataTables/dt_Feat_Table.dt_Feat_Table")
  (Class|ModController|MergeDataTables "/Game/Items/ItemTable.ItemTable" "/Game/Mods/Profession_and_Mastery/DataTables/dt_Class_Mastery_Item_Table.dt_Class_Mastery_Item_Table")
  (Class|ModController|MergeDataTables "/Game/Items/Recipes/RecipesTable.RecipesTable" "/Game/Mods/Profession_and_Mastery/DataTables/dt_Class_Mastery_Recipe_Table.dt_Class_Mastery_Recipe_Table")
  (Class|ModController|MergeDataTables "/Game/Systems/SpawnTable/ProfessionTemplateDataTable.ProfessionTemplateDataTable" "/Game/Mods/Profession_and_Mastery/DataTables/dt_Profession_Template_Table.dt_Profession_Template_Table")
  (Class|ModController|MergeDataTables "/Game/Items/ItemStatModificationTable.ItemStatModificationTable" "/Game/Mods/Profession_and_Mastery/DataTables/dt_custom_item_modif.dt_custom_item_modif")
  (Class|ModController|MergeDataTables "/Game/Items/EquipmentVariationTable.EquipmentVariationTable" "/Game/Mods/Profession_and_Mastery/DataTables/dt_custom_equip_var.dt_custom_equip_var")
  (Class|ModController|MergeDataTables "/Game/Items/ItemStatModificationTable.ItemStatModificationTable" "/Game/Mods/Profession_and_Mastery/DataTables/dt_OW_ItemStatModificationTable.dt_OW_ItemStatModificationTable")
  (Class|ModController|MergeDataTables "/Game/UI/CharacterCreation/DataTables/EyeMakeupColorSelections.EyeMakeupColorSelections" "/Game/Mods/Profession_and_Mastery/DataTables/dt_corrupted_colours.dt_corrupted_colours")
  (Class|ModController|MergeDataTables "/Game/UI/CharacterCreation/DataTables/LipMakeupColorSelections.LipMakeupColorSelections" "/Game/Mods/Profession_and_Mastery/DataTables/dt_corrupted_colours.dt_corrupted_colours")
  (Class|ModController|MergeDataTables "/Game/Items/ItemStatModificationTable.ItemStatModificationTable" "/Game/Mods/Profession_and_Mastery/DataTables/dt_OW_DLC_ItemStatModificationTable.dt_OW_DLC_ItemStatModificationTable")
  (Class|ModController|MergeDataTables "/Game/Items/ItemStatModificationTable.ItemStatModificationTable" "/Game/Mods/Profession_and_Mastery/DataTables/dt_Primal_Stat_Overwrite.dt_Primal_Stat_Overwrite")
  (Class|ModController|MergeDataTables "/Game/Items/ItemStatModificationTable.ItemStatModificationTable" "/Game/Mods/Profession_and_Mastery/DataTables/dt_OW_DLC2_ItemStatModificationTable.dt_OW_DLC2_ItemStatModificationTable")
  (Class|ModController|MergeDataTables "/Game/Items/Recipes/RecipesTable.RecipesTable")
  (Class|ModController|MergeDataTables "/Game/Items/Feats/FeatTable.FeatTable")
  (Class|ModController|MergeDataTables "/Game/Items/ItemTable.ItemTable" "/Game/Mods/Profession_and_Mastery/DataTables/New_tables_TigeR/DT_Loot_AC_Item.DT_Loot_AC_Item")
  (Class|ModController|MergeDataTables "/Game/Items/ItemStatModificationTable.ItemStatModificationTable" "/Game/Mods/Profession_and_Mastery/DataTables/dt_OW_DLC3_ItemStatModificationTable.dt_OW_DLC3_ItemStatModificationTable")
  (Class|ModController|MergeDataTables "/Game/Items/ItemTable.ItemTable" "/Game/Mods/Profession_and_Mastery/DataTables/New_tables_TigeR/DT_Loot_AC_Item.DT_Loot_AC_Item")
  (Class|ModController|MergeDataTables "/Game/Items/ItemStatModificationTable.ItemStatModificationTable" "/Game/Mods/Profession_and_Mastery/DataTables/New_tables_TigeR/DT_LOOT_AC_ModificationTable.DT_LOOT_AC_ModificationTable")
  (Class|ModController|MergeDataTables "/Game/Items/ItemStatModificationTable.ItemStatModificationTable" "/Game/Mods/Profession_and_Mastery/DataTables/dt_OW_DLC4_ItemStatModificationTable.dt_OW_DLC4_ItemStatModificationTable")
  (Class|ModController|MergeDataTables "/Game/Systems/Survival/Gathering/Gathering_v2/ItemNameToTemplateID.ItemNameToTemplateID" "/Game/Mods/Profession_and_Mastery/DataTables/dt_CM_ItemnametoTemplateID.dt_CM_ItemnametoTemplateID")
  (Class|ModController|MergeDataTables "/Game/Systems/Survival/Gathering/Gathering_v2/LootTable_Resource.LootTable_Resource" "/Game/Mods/Profession_and_Mastery/DataTables/dt_CM_LootTable_Resource.dt_CM_LootTable_Resource")
  (Class|ModController|MergeDataTables "/Game/Systems/Progression/DT_ExilesJourney.DT_ExilesJourney" "/Game/Mods/Profession_and_Mastery/DataTables/dt_CM_journey.dt_CM_journey")
  (Class|ModController|MergeDataTables "/Game/Items/ItemTable.ItemTable" "/Game/Mods/Profession_and_Mastery/DataTables/dt_Class_Mastery_ItemTable_02.dt_Class_Mastery_ItemTable_02")
  (Class|ModController|MergeDataTables "/Game/UI/CharacterCreation/DataTables/Male_WarPaintSelections.Male_WarPaintSelections" "/Game/Mods/Profession_and_Mastery/DataTables/Legendary_Warpaint_set_Male.Legendary_Warpaint_set_Male")
  (Class|ModController|MergeDataTables "/Game/UI/CharacterCreation/DataTables/Female_WarPaintSelections.Female_WarPaintSelections" "/Game/Mods/Profession_and_Mastery/DataTables/Legendary_Warpaint_set_Female.Legendary_Warpaint_set_Female")
  (Class|ModController|MergeDataTables "/Game/Items/ItemStatModificationTable.ItemStatModificationTable" "/Game/Mods/Profession_and_Mastery/DataTables/dt_Warpaint_StatModificationTable.dt_Warpaint_StatModificationTable")
  (Class|ModController|MergeDataTables "/Game/Systems/Loot/TableSetup/W_Loot_AbandonedCity_TheBruteBoss.W_Loot_AbandonedCity_TheBruteBoss" "/Game/Mods/Profession_and_Mastery/DataTables/Loot_tables/W_Loot_AbandonedCity_Warpaints.W_Loot_AbandonedCity_Warpaints")
  (Class|ModController|MergeDataTables "/Game/Systems/Loot/TableSetup/W_Loot_AbandonedCity_RedMotherBoss.W_Loot_AbandonedCity_RedMotherBoss" "/Game/Mods/Profession_and_Mastery/DataTables/Loot_tables/W_Loot_AbandonedCity_Warpaints.W_Loot_AbandonedCity_Warpaints")
  (Class|ModController|MergeDataTables "/Game/Systems/Loot/TableSetup/W_Loot_AbandonedCity_SkeletonBoss.W_Loot_AbandonedCity_SkeletonBoss" "/Game/Mods/Profession_and_Mastery/DataTables/Loot_tables/W_Loot_AbandonedCity_Warpaints.W_Loot_AbandonedCity_Warpaints")
  (Class|ModController|MergeDataTables "/Game/Systems/Loot/TableSetup/W_Loot_AbandonedCity_WingedDeathBoss.W_Loot_AbandonedCity_WingedDeathBoss" "/Game/Mods/Profession_and_Mastery/DataTables/Loot_tables/W_Loot_AbandonedCity_Warpaints.W_Loot_AbandonedCity_Warpaints")
  (Class|ModController|MergeDataTables "/Game/Items/ItemTable.ItemTable" "/Game/Mods/Profession_and_Mastery/DataTables/dt_Class_Token_itemtable.dt_Class_Token_itemtable")
  (Class|ModController|MergeDataTables "/Game/Systems/SpawnTable/SpawnDataTable.SpawnDataTable" "/Game/Mods/Profession_and_Mastery/DataTables/Thralls/dt_Class_thrall_SpawnDataTable.dt_Class_thrall_SpawnDataTable")
  (Class|ModController|MergeDataTables "/Game/Items/ItemTable.ItemTable" "/Game/Mods/Profession_and_Mastery/DataTables/Legendary_Armour_Tables/dt_Class_LegendaryArmour_ItemTable_light.dt_Class_LegendaryArmour_ItemTable_light")
  (Class|ModController|MergeDataTables "/Game/Items/ItemStatModificationTable.ItemStatModificationTable" "/Game/Mods/Profession_and_Mastery/DataTables/Legendary_Armour_Tables/dt_Class_Legend_light_Stats.dt_Class_Legend_light_Stats")
  (Class|ModController|MergeDataTables "/Game/Items/EquipmentVariationTable.EquipmentVariationTable" "/Game/Mods/Profession_and_Mastery/DataTables/Legendary_Armour_Tables/dt_Class_Legend_light_equipvar.dt_Class_Legend_light_equipvar")
  (Class|ModController|MergeDataTables "/Game/Items/ItemStatModificationTable.ItemStatModificationTable" "/Game/Mods/Profession_and_Mastery/DataTables/dt_OW_DLC5_ItemStatModificationTable2.dt_OW_DLC5_ItemStatModificationTable2")
  (Class|ModController|MergeDataTables "/Game/Items/ItemStatModificationTable.ItemStatModificationTable" "/Game/Mods/Profession_and_Mastery/DataTables/Legendary_Armour_Tables/dt_class_Legend_heavy_itemstatmodification.dt_class_Legend_heavy_itemstatmodification")
  (Class|ModController|MergeDataTables "/Game/Items/ItemStatModificationTable.ItemStatModificationTable" "/Game/Mods/Profession_and_Mastery/DataTables/Legendary_Armour_Tables/dt_class_Legend_Medium_statmodificationtable.dt_class_Legend_Medium_statmodificationtable")
  (Class|ModController|MergeDataTables "/Game/Items/EquipmentVariationTable.EquipmentVariationTable" "/Game/Mods/Profession_and_Mastery/DataTables/Legendary_Armour_Tables/dt_class_Legend_Medium_EquipmentVarTable.dt_class_Legend_Medium_EquipmentVarTable")
  (Class|ModController|MergeDataTables "/Game/Items/EquipmentVariationTable.EquipmentVariationTable" "/Game/Mods/Profession_and_Mastery/DataTables/Legendary_Armour_Tables/dt_Class_Legend_Heavy_equipvartable.dt_Class_Legend_Heavy_equipvartable")
  (Class|ModController|MergeDataTables "/Game/Items/ItemTable.ItemTable" "/Game/Mods/Profession_and_Mastery/DataTables/Legendary_Armour_Tables/dt_Class_Legend_Medium_itemtable.dt_Class_Legend_Medium_itemtable")
  (Class|ModController|MergeDataTables "/Game/Items/ItemTable.ItemTable" "/Game/Mods/Profession_and_Mastery/DataTables/Legendary_Armour_Tables/dt_class_Legend_Heavy_itemtable.dt_class_Legend_Heavy_itemtable")
  (Class|ModController|MergeDataTables "/Game/Items/Feats/FeatTable.FeatTable" "/Game/Mods/Profession_and_Mastery/DataTables/Legendary_Armour_Tables/dt_Class_Legend_FeatTable.dt_Class_Legend_FeatTable")
  (Class|ModController|MergeDataTables "/Game/Items/Recipes/RecipesTable.RecipesTable" "/Game/Mods/Profession_and_Mastery/DataTables/Legendary_Armour_Tables/dt_class_Legend_RecipeTable.dt_class_Legend_RecipeTable")
  (Class|ModController|MergeDataTables "/Game/Systems/Progression/DT_FeatsPerLevel.DT_FeatsPerLevel" "/Game/Mods/Profession_and_Mastery/DataTables/Legendary_Armour_Tables/DT_FeatsPerLevel_class.DT_FeatsPerLevel_class")
  (Class|ModController|MergeDataTables "/Game/Items/Crafting/CraftingStationNameTable.CraftingStationNameTable" "/Game/Mods/Profession_and_Mastery/DataTables/Legendary_Armour_Tables/dt_Class_craftingstationname.dt_Class_craftingstationname")
  (Class|ModController|MergeDataTables "/Game/Items/ItemTable.ItemTable" "/Game/Mods/Profession_and_Mastery/DataTables/Legendary_Armour_Tables/dt_class_OtherArmour_itemtable.dt_class_OtherArmour_itemtable")
  (Class|ModController|MergeDataTables "/Game/Items/EquipmentVariationTable.EquipmentVariationTable" "/Game/Mods/Profession_and_Mastery/DataTables/Legendary_Armour_Tables/dt_OtherA_EquipVar.dt_OtherA_EquipVar")
  (Class|ModController|MergeDataTables "/Game/Items/ItemStatModificationTable.ItemStatModificationTable" "/Game/Mods/Profession_and_Mastery/DataTables/Legendary_Armour_Tables/dt_Itemstatmodification_OtherArmour.dt_Itemstatmodification_OtherArmour")
  (Class|ModController|MergeDataTables "/Game/Items/ItemStatModificationTable.ItemStatModificationTable" "/Game/Mods/Profession_and_Mastery/DataTables/DT_OW_DLC6_riddle_ItemStatModification.DT_OW_DLC6_riddle_ItemStatModification")
  (Class|ModController|MergeDataTables "/Game/Systems/Survival/Gathering/Gathering_v2/LootTable_Resource.LootTable_Resource" "/Game/Mods/Profession_and_Mastery/DataTables/dt_CM_LootTable_Resource.dt_CM_LootTable_Resource")
  (Class|ModController|MergeDataTables "/Game/Systems/SpawnTable/ProfessionTemplateDataTable.ProfessionTemplateDataTable" "/Game/Mods/Profession_and_Mastery/DataTables/dt_Profession_Template_Table.dt_Profession_Template_Table")
  (Class|ModController|MergeDataTables "/Game/Characters/NPCs/MonsterStatTable.MonsterStatTable" "/Game/Mods/Profession_and_Mastery/DataTables/dt_Monsterstattable_CM.dt_Monsterstattable_CM")
  (Class|ModController|MergeDataTables "/Game/Systems/Thrall/ThrallDataTable.ThrallDataTable" "/Game/Mods/Profession_and_Mastery/DataTables/dt_thrall_DataTable.dt_thrall_DataTable"))

(fn Widget)